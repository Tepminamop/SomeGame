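; Arrow actor that serves as a player pickup and as a bow-fired projectile.
; A state machine (Unobtained, In Bow, In Air) sets collision, adding projectile movement on firing with speed scaled by bow charge and removing it on leaving flight.
; Overlaps give an unobtained arrow to the first-person character, or destroy a flying one unless it hits the player or an Interact implementer.
; Logic to stick arrows into hit actors is disconnected, noted as broken.
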(event `Fire`
  (params (BowCharge :type "Float (double-precision)"))
  (set `self.BowCharge` BowCharge)
  (`self.SetArrowState` "NewEnumerator2"))

(event `self.ArrowMesh.OnComponentBeginOverlap`
  (params (OverlappedComponent :type "PrimitiveComponent Object Reference") (OtherActor :type "Actor Object Reference") (OtherComp :type "PrimitiveComponent Object Reference") (OtherBodyIndex :type Integer) (bFromSweep :type Boolean) (SweepResult :type "HitResult Structure (by ref)"))
  (`KismetSystemLibrary.PrintString` "Begin Overlap")
  (`self.HandleOverlap` OtherActor SweepResult))

(fn `HandleOverlap`
  (params (OtherActor :type "Actor Object Reference") (HitResult :type "HitResult Structure"))
  (switch `/Game/MyStuff/BluePrints/EArrowState` (`self.ArrowState`)
    (:`NewEnumerator0`
      (bind _asbp_first_person_character (cast `/Game/FirstPerson/Blueprints/BP_FirstPersonCharacter` OtherActor))
      (`/Game/FirstPerson/Blueprints/BP_FirstPersonCharacter.AddArrows` _asbp_first_person_character 1)
      (`self.K2_DestroyActor`))
    (:`NewEnumerator2`
      (if (!= (`local.OtherActor`) (`GameplayStatics.GetPlayerCharacter` 0))
        (if (not (`KismetSystemLibrary.DoesImplementInterface` (`local.OtherActor`) "/Game/InventorySystem/Migrate/Interact.Interact_C"))
          (`self.K2_DestroyActor`))))))

(fn `OnStateBegin`
  (params (State :type "/Game/MyStuff/BluePrints/EArrowState Enum" :default "NewEnumerator0"))
  (switch `/Game/MyStuff/BluePrints/EArrowState` State
    (:`NewEnumerator0`
      (`PrimitiveComponent.SetCollisionProfileName` (`self.ArrowMesh`) "OverlapAllDynamic" true))
    (:`NewEnumerator1`
      (`PrimitiveComponent.SetCollisionProfileName` (`self.ArrowMesh`) "NoCollision" true))
    (:`NewEnumerator2`
      (`PrimitiveComponent.SetCollisionProfileName` (`self.ArrowMesh`) "OverlapAllDynamic" true)
      (bind _returnvalue (`AddComponent|NODE_AddProjectileMovementComponent-0`))
      (bind _output_get (set `self.ProjectileComponent` _returnvalue))
      (set `MovementComponent.Velocity` (* (`self.GetActorForwardVector`) (`KismetMathLibrary.Lerp` 100.0 4000.0 (`self.BowCharge`))) _output_get)
      (set `ProjectileMovementComponent.bRotationFollowsVelocity` true _output_get))))

(fn `OnStateEnd`
  (params (State :type "/Game/MyStuff/BluePrints/EArrowState Enum" :default "NewEnumerator0"))
  (switch `/Game/MyStuff/BluePrints/EArrowState` State
    (:`NewEnumerator2`
      (`ActorComponent.K2_DestroyComponent` (`self.ProjectileComponent`)))))

(fn `SetArrowState`
  (params (`New state` :type "/Game/MyStuff/BluePrints/EArrowState Enum" :default "NewEnumerator0"))
  (if (`|EnumInequality` `New state` (`self.ArrowState`))
    (`self.OnStateEnd` (`self.ArrowState`))
    (bind _output_get (set `self.ArrowState` (`local.New state`)))
    (`self.OnStateBegin` _output_get)))

(fn `UserConstructionScript`
  (`SceneComponent.SetRelativeScale3D` (`self.ArrowMesh`) (1.0 5.0 5.0)))