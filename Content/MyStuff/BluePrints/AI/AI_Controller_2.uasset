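; AI controller that makes its pawn wander endlessly between random navmesh locations.
; BeginPlay picks a nearby navigable point and calls the custom Restart event, which runs AIMoveTo.
; On success it stops, waits briefly, picks a reachable point in a wider radius and calls itself again; failed moves are not handled.
; Unconnected leftover experiments cover TargetPoint cycling, navmesh raycasts and simple move nodes.
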(event `self.ReceiveTick`
  (params (DeltaSeconds :type "Float (single-precision)"))
  ;[1 1 1] Rycling between random locations
)

(event `self.ReceiveBeginPlay`
  ;[1 1 1] Better cycling between random locations
  (bind _randomlocation (`NavigationSystemV1.K2_GetRandomLocationInNavigableRadius` (`self.K2_GetActorLocation` (`self.K2_GetPawn`)) 400.0 null null))
  (set `self.RandomPoint` _randomlocation)
  (`self.Restart`))

(event `Restart`
  ;[1 1 1] Better cycling between random locations
  (`|AIMoveTo` null (`self.RandomPoint`) null
    (:`OnSuccess`
      (`KismetSystemLibrary.PrintString` "Finish")
      (`self.StopMovement`)
      (`KismetSystemLibrary.Delay` 2.0)
      (set `self.RandomPoint` (`NavigationSystemV1.K2_GetRandomReachablePointInRadius` (`self.K2_GetActorLocation` (`self.K2_GetPawn`)) 3000.0 null null))
      (`self.Restart`))))

(fn `UserConstructionScript`)