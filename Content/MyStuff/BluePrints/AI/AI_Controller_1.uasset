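; AI controller that makes its pawn wander while steering away from obstacles, using a simple eyes, brain and legs loop on Tick.
; A horizontal visibility line trace along the pawn's forward vector detects blockers, with debug drawing on.
; Each blocked frame yaws the stored Direction by a small step, randomly left or right.
; Movement input is applied along Direction every frame, whether blocked or not.
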(event `self.ReceiveTick`
  (params (DeltaSeconds :type "Float (single-precision)"))
  (bind _returnvalue (`self.K2_GetPawn`))
  (bind _returnvalue_2 (`self.K2_GetActorLocation` _returnvalue))
  ;[1 1 1] Eyes
  (bind (_outhit _returnvalue_3) (`KismetSystemLibrary.LineTraceSingle` :`Start` _returnvalue_2 :`End` (+ _returnvalue_2 (* (`self.GetActorForwardVector` _returnvalue) (800.0 800.0 0.0))) :`TraceChannel` "TraceTypeQuery1" :`DrawDebugType` "ForOneFrame"))
  ;[1 1 1] Brain
  (if _returnvalue_3
    (set `self.RandomDirection` (select `bool` (`KismetMathLibrary.RandomBool`) :`false` 10.0 :`true` -10.0))
    (set `self.Direction` (`KismetMathLibrary.GreaterGreater_VectorRotator` (`self.Direction`) (`KismetMathLibrary.MakeRotator` 0.0 0.0 (`self.RandomDirection`)))))
  ;[1 1 1] Legs
  (`Pawn.AddMovementInput` _returnvalue (`self.Direction`) 1.0 false))

(fn `UserConstructionScript`)