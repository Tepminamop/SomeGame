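; BP_Bow is a bow actor that charges, fires and reloads BP_Arrow projectiles.
; A timeline drives ChargeAmount while charging, plays in reverse when charging ends, and is stopped and reset after each shot.
; Fire detaches the held arrow, passes it the current charge and clears the reference.
; Reload spawns a new arrow and attaches it to the bow mesh's arrow socket.
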(event `BeginCharge`
  (`self.Arrow`
    (:`then`
      (bind (_direction _chrgeamount) (`Timeline|ChrgeTimeline` :!label _label)
        (:`Update`
          (set `self.ChargeAmount` _chrgeamount))))
    (:`else`)))

(event `StopCharge`
  (`|ExecutionSequence`
    (:`then_0`
      (goto _label :!via `Stop`))
    (:`then_1`
      (goto _label :!via `SetNewTime`))))

(event `EndCharge`
  (`self.Arrow`
    (:`then`
      (goto _label :!via `Reverse`))
    (:`else`)))

(event `Fire`
  (bind _arrow (`self.Arrow`)
    (:`then`
      (`self.K2_DetachFromActor` _arrow "KeepWorld" "KeepWorld" "KeepWorld")
      (`/Game/MyStuff/BluePrints/Bow_Arrow/BP_Arrow.Fire` (`self.Arrow`) (`self.ChargeAmount`))
      (set `self.Arrow` null)
      (`self.StopCharge`))
    (:`else`)))

(event `Reload`
  (bind _returnvalue (`|SpawnActorFromClass` "/Game/MyStuff/BluePrints/Bow_Arrow/BP_Arrow.BP_Arrow_C" (`KismetMathLibrary.MakeTransform` (0.0 0.0 0.0)) "Undefined" "OverrideRootScale" null "NewEnumerator1" null))
  (bind _output_get (set `self.Arrow` _returnvalue))
  (`self.K2_AttachToComponent` _output_get (`self.BowMesh`) "arrow_attach_socket" "SnapToTarget" "SnapToTarget" "KeepWorld" true))

(fn `UserConstructionScript`)